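; AI_BP is a wheeled vehicle Blueprint, named for AI use, that updates gear state and engine audio, with no driving logic in its graphs.
; Each Tick it sets a reverse-gear flag from the current gear and feeds absolute forward speed, rather than engine RPM, into the engine sound's RPM parameter.
; An unconnected Car Recovery chain that would teleport and re-orient the mesh never runs.
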(event `self.ReceiveBeginPlay`)

(event `self.ReceiveTick`
  (params (DeltaSeconds :type "Float (single-precision)"))
  ;[1 1 1] Update
  (`|ExecutionSequence`
    (:`then_0`
      (set `self.InReverseGear` (< (`WheeledVehicleMovementComponent.GetCurrentGear` (`self.VehicleMovement`)) 0)))
    (:`then_1`
      ;[1 1 1] Audio
      (`AudioComponent.SetFloatParameter` (`self.EngineSound`) "RPM" (`KismetMathLibrary.Abs` (`WheeledVehicleMovementComponent.GetForwardSpeed` (`self.VehicleMovement`)))))))

(fn `UserConstructionScript`)