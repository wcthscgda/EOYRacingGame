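; AI vehicle Blueprint, apparently an unfinished AI-driven car with no steering or throttle logic in its graphs.
; Tick flags reverse gear from the vehicle movement and feeds absolute forward speed into the engine sound's RPM parameter.
; Mesh overlaps with AI_Turns actors only print debug strings while checking the Turns array.
; An unconnected car recovery snippet would teleport the mesh in place with a rebuilt rotation, but never runs.
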(event `self.ReceiveBeginPlay`)

(event `self.ReceiveTick`
  (params (DeltaSeconds :type "Float (single-precision)"))
  ;[1 1 1] Update
  (`|ExecutionSequence`
    (:`then_0`
      (set `self.InReverseGear` (< (`WheeledVehicleMovementComponent.GetCurrentGear` (`self.VehicleMovement`)) 0)))
    (:`then_1`
      ;[1 1 1] Audio
      (`AudioComponent.SetFloatParameter` (`self.EngineSound`) "RPM" (`KismetMathLibrary.Abs` (`WheeledVehicleMovementComponent.GetForwardSpeed` (`self.VehicleMovement`)))))))

(event `self.Mesh.OnComponentBeginOverlap`
  (params (OverlappedComponent :type "PrimitiveComponent Object Reference") (OtherActor :type "Actor Object Reference") (OtherComp :type "PrimitiveComponent Object Reference") (OtherBodyIndex :type Integer) (bFromSweep :type Boolean) (SweepResult :type "HitResult Structure (by ref)"))
  (bind _asai_turns (cast `/Game/1_Blueprints_VehicleAdvBP/Blueprints/AI/AI_Turns` OtherActor)
    (:`then`
      (for _array_element (`/Game/1_Blueprints_VehicleAdvBP/Blueprints/AI/AI_Turns.Turns` _asai_turns)
        (if (== _array_element OtherActor)
          (`KismetSystemLibrary.PrintString` "succsess")
          (else
            (`KismetSystemLibrary.PrintString` "Stage 2")))))
    (:`CastFailed`
      (`KismetSystemLibrary.PrintString` "Stage 1"))))

(fn `UserConstructionScript`)